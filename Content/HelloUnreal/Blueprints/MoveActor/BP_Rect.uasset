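; BP_Rect is an actor that moves its Cube along a looping, axis-aligned path defined by the MoveSequence array, toggled by PlayAction.
; Each Tick, Move offsets the Cube's relative location by MoveSpeed until it reaches MovingDistance, then calls CheckStep.
; CheckStep folds that offset into the actor location and zeroes the Cube before the next step, but skips this when wrapping to the first.
; A Timeline-based movement alternative is left unconnected.
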(event Custom|CheckStep
  ;[0.15 0.15 0.15 0.5] Comment
  (bind _result (Math|Integer|IncrementInt (Variables|Default|GetCurrentStep))
    (:%20%20
      (if (<= _result (Variables|Default|GetMaxStep))
        (Variables|Default|SetMoveType (Utilities|Array|Get(acopy) (Variables|Default|GetMoveSequence) (Variables|Default|GetCurrentStep)))
        (Transformation|SetActorLocation (+ (Transformation|GetActorLocation) (Variables|/Script/Engine.SceneComponent|GetRelativeLocation (Variables|Default|GetCube))) false false)
        (Transformation|SetRelativeLocation (Variables|Default|GetCube) "0, 0, 0" false false)
        (else
          (bind _output_get (Variables|Default|SetCurrentStep 0))
          (Variables|Default|SetMoveType (Utilities|Array|Get(acopy) (Variables|Default|GetMoveSequence) _output_get)))))))

(event Custom|Move
  (if (Variables|Default|GetIsMoving)
    (switch Utilities|FlowControl|Switch|SwitchonE_MoveType (Variables|Default|GetMoveType)
      (:NewEnumerator0
        ;[0.15 0.15 0.15 0.5] Right
        (Transformation|AddRelativeLocation (Variables|Default|GetCube) (Math|Vector|MakeVector 0.0 (Variables|Default|GetMoveSpeed) 0.0) false false)
        (if (>= (.y (Variables|/Script/Engine.SceneComponent|GetRelativeLocation (Variables|Default|GetCube))) (Variables|Default|GetMovingDistance))
          (CallFunction|CheckStep)))
      (:NewEnumerator1
        ;[0.15 0.15 0.15 0.5] Left
        (Transformation|AddRelativeLocation (Variables|Default|GetCube) (Math|Vector|MakeVector 0.0 (* (Variables|Default|GetMoveSpeed) -1.0) 0.0) false false)
        (if (<= (.y (Variables|/Script/Engine.SceneComponent|GetRelativeLocation (Variables|Default|GetCube))) (* (Variables|Default|GetMovingDistance) -1.0))
          (CallFunction|CheckStep)))
      (:NewEnumerator2
        ;[0.15 0.15 0.15 0.5] Forward
        (Transformation|AddRelativeLocation (Variables|Default|GetCube) (Math|Vector|MakeVector (Variables|Default|GetMoveSpeed) 0.0 0.0) false false)
        (if (>= (.x (Variables|/Script/Engine.SceneComponent|GetRelativeLocation (Variables|Default|GetCube))) (Variables|Default|GetMovingDistance))
          (CallFunction|CheckStep)))
      (:NewEnumerator3
        ;[0.15 0.15 0.15 0.5] Backward
        (Transformation|AddRelativeLocation (Variables|Default|GetCube) (Math|Vector|MakeVector (* (Variables|Default|GetMoveSpeed) -1.0) 0.0 0.0) false false)
        (if (<= (.x (Variables|/Script/Engine.SceneComponent|GetRelativeLocation (Variables|Default|GetCube))) (* (Variables|Default|GetMovingDistance) -1.0))
          (CallFunction|CheckStep)))
      (:NewEnumerator4
        ;[0.15 0.15 0.15 0.5] Up
        (Transformation|AddRelativeLocation (Variables|Default|GetCube) (Math|Vector|MakeVector 0.0 0.0 (Variables|Default|GetMoveSpeed)) false false)
        (if (>= (.z (Variables|/Script/Engine.SceneComponent|GetRelativeLocation (Variables|Default|GetCube))) (Variables|Default|GetMovingDistance))
          (CallFunction|CheckStep)))
      (:NewEnumerator5
        ;[0.15 0.15 0.15 0.5] Down
        (Transformation|AddRelativeLocation (Variables|Default|GetCube) (Math|Vector|MakeVector 0.0 0.0 (* (Variables|Default|GetMoveSpeed) -1.0)) false false)
        (if (<= (.z (Variables|/Script/Engine.SceneComponent|GetRelativeLocation (Variables|Default|GetCube))) (* (Variables|Default|GetMovingDistance) -1.0))
          (CallFunction|CheckStep))))))

(event EventTick
  (params (DeltaSeconds :type Float%20%28single-precision%29))
  ;[0.15 0.15 0.15 0.5] Comment
  (CallFunction|Move))

(event EventPlayAction
  (params (IsPlay :type Boolean))
  (Variables|Default|SetIsMoving IsPlay))

(event EventBeginPlay
  (bind _movesequence (Variables|Default|GetMoveSequence))
  (bind _returnvalue (Utilities|Array|Length _movesequence))
  ;[0.15 0.15 0.15 0.5] Comment
  (if (> _returnvalue 0)
    (Variables|Default|SetMaxStep (- _returnvalue 1))
    (Variables|Default|SetMoveType (Utilities|Array|Get(acopy) (Variables|Default|GetMoveSequence) (Variables|Default|GetCurrentStep)))))

(fn ConstructionScript)