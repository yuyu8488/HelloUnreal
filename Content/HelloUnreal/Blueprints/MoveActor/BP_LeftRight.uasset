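; A toggleable moving actor that shuttles its Cube back and forth along its local Y axis.
; Tick calls Move, which, while IsMoving is set by PlayAction, offsets the Cube by MoveSpeed per frame without delta time scaling.
; ChangeDirection flips once the Cube reaches plus or minus MovingDistance.
; An alternative Timeline-based actor movement and a SetRelativeLocation snippet sit unconnected.
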(event Custom|Move
  ;[0.15 0.15 0.15 0.5] Move
  (if (Variables|Default|GetIsMoving)
    (if (Variables|Default|GetChangeDirection)
      (Transformation|AddRelativeLocation (Variables|Default|GetCube) (Math|Vector|MakeVector 0.0 (* (Variables|Default|GetMoveSpeed) -1.0) 0.0) false false)
      (if (<= (.y (Variables|/Script/Engine.SceneComponent|GetRelativeLocation (Variables|Default|GetCube))) (* (Variables|Default|GetMovingDistance) -1.0))
        (Variables|Default|SetChangeDirection false))
      (else
        (Transformation|AddRelativeLocation (Variables|Default|GetCube) (Math|Vector|MakeVector 0.0 (Variables|Default|GetMoveSpeed) 0.0) false false)
        (if (>= (.y (Variables|/Script/Engine.SceneComponent|GetRelativeLocation (Variables|Default|GetCube))) (Variables|Default|GetMovingDistance))
          (Variables|Default|SetChangeDirection true))))))

(event EventTick
  (params (DeltaSeconds :type Float%20%28single-precision%29))
  (CallFunction|Move))

(event EventPlayAction
  (params (IsPlay :type Boolean))
  (Variables|Default|SetIsMoving IsPlay))

(fn ConstructionScript)

(fn NewFunction)