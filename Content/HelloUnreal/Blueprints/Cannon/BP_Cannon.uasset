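; BP_Cannon is a cannon actor that toggles continuous firing of BP_CannonBall from its Arrow component's location and rotation.
; On BeginPlay it binds to the toggle-interact event of its BPSwitch reference, printing a warning if that is unset.
; PlayAction flips the firing state, either spawning immediately and starting a looping spawn timer or clearing it.
; A separate ClearTimerHandle event also stops the timer.
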(event EventPlayAction
  (params (IsPlay :type Boolean))
  (CallFunction|ShootCannonBall))

(event EventClearTimerHandle
  (Utilities|Time|ClearandInvalidateTimerbyHandle (Variables|Default|GetShootCannonBallTimer)))

(event EventBeginPlay
  (bind _bp_switch (Variables|Default|GetBP_Switch)
    (:then
      (EventDispatchers|BindEventtoOnToggleInteractActor _bp_switch (EventDispatchers|CreateEvent :!event PlayAction)))
    (:else
      (Development|PrintString "BP_Swich is nullptr"))))

(fn ConstructionScript)

(fn SpawnCannonBall
  (bind _arrow (Variables|Default|GetArrow))
  (bind _returnvalue (Transformation|GetWorldTransform _arrow))
  (Game|SpawnActorfromClass "/Game/HelloUnreal/Blueprints/Cannon/BP_CannonBall.BP_CannonBall_C" (Math|Transform|MakeTransform (.location _returnvalue) (.rotation _returnvalue) "1.000000,1.000000,1.000000") "AlwaysSpawn" "MultiplyWithRoot" 0 0))

(fn ShootCannonBall
  (Variables|Default|SetToggle (not (Variables|Default|GetToggle)))
  (if (Variables|Default|GetToggle)
    (if (not (Class|KismetSystemLibrary|TimerExistsHandle (Variables|Default|GetShootCannonBallTimer)))
      (CallFunction|SpawnCannonBall)
      (bind _returnvalue (Utilities|Time|SetTimerbyFunctionName 0 "SpawnCannonBall" 1.0 true))
      (Variables|Default|SetShootCannonBallTimer _returnvalue))
    (else
      (Utilities|Time|ClearandInvalidateTimerbyHandle (Variables|Default|GetShootCannonBallTimer)))))