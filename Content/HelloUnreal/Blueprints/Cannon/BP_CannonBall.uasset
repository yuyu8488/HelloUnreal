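; BP_CannonBall is a physics projectile that explodes on impact and knocks characters back.
; On BeginPlay it launches the Ball component along the actor's forward vector with a large impulse and sets a short lifespan as a fallback.
; A hit spawns a pooled explosion effect, pushes any hit Character's movement component using the scaled, inverted normal impulse, and destroys the actor after a brief delay.
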(event OnComponentHit(Ball)
  (params (HitComponent :type Primitive%20Component%20Object%20Reference) (OtherActor :type Actor%20Object%20Reference) (OtherComp :type Primitive%20Component%20Object%20Reference) (NormalImpulse :type Vector :default "0, 0, 0") (Hit :type Hit%20Result%20Structure%20%28by%20ref%29))
  (Utilities|FlowControl|Sequence
    (:then_0
      ;[0.15 0.15 0.15 0.5] VFX
      (Effects|SpawnEmitteratLocation "/Game/StarterContent/Particles/P_Explosion.P_Explosion" (.Location (Collision|BreakHitResult Hit)) "0, 0, 0" "1.000000,1.000000,1.000000" true "AutoRelease")
      (Utilities|FlowControl|Delay 1.0)
      (Actor|DestroyActor))
    (:then_1
      (bind _ascharacter (Utilities|Casting|CastToCharacter OtherActor))
      (Physics|AddImpulse (Variables|/Script/Engine.Character|GetCharacterMovement _ascharacter) (* NormalImpulse -0.1) true))))

(event EventBeginPlay
  (Physics|AddImpulse (Variables|Default|GetBall) (* (Transformation|GetActorForwardVector) 8e+04) "None" false)
  (Actor|SetLifeSpan 5.0))

(fn ConstructionScript)