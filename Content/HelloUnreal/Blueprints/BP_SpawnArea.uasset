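; BP_SpawnArea is a box-bounded area that spawns batches of actors at random points inside its volume.
; Its DoSomething event waits briefly, then runs two spawn loops in sequence: one for the class in SpawnActorClass, one for a larger batch of BP_RedBall.
; Each spawn picks a random point within the Box component's scaled extent and always spawns regardless of collision.
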(event Custom|Do%20Something
  (bind _box (Variables|Default|GetBox))
  (bind _box_2 (Variables|Default|GetBox))
  (Utilities|FlowControl|Delay 1.0)
  (Utilities|FlowControl|Sequence
    (:then_0
      (for _index (range 0 4)
        (Game|SpawnActorfromClass (Variables|Default|GetSpawnActorClass) (Math|Transform|MakeTransform (Math|Random|RandomPointinBoundingBox (Transformation|GetWorldLocation _box_2) (Components|Box|GetScaledBoxExtent _box_2)) "0, 0, 0" "1.000000,1.000000,1.000000") "AlwaysSpawn" "MultiplyWithRoot" 0 0)))
    (:then_1
      (for _index_2 (range 0 9)
        (Game|SpawnActorfromClass "/Game/HelloUnreal/Blueprints/BP_RedBall.BP_RedBall_C" (Math|Transform|MakeTransform (Math|Random|RandomPointinBoundingBox (Transformation|GetWorldLocation _box) (Components|Box|GetScaledBoxExtent _box)) "0, 0, 0" "1.000000,1.000000,1.000000") "AlwaysSpawn" "MultiplyWithRoot" 0 0)))))

(fn ConstructionScript)