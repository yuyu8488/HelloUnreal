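; BP_Timer is a timer Blueprint that shows an accumulated HH:MM:SS clock on its TextRender.
; PlayAction starts or pauses it, and while it runs, Tick adds delta time scaled by Speed to the running total.
; FloatToString00 pads each field to two digits.
; The hour and minute divisors (8640, 360) are not standard time conversions, so the fields do not roll over like a real clock.
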(event Custom|Run
  (params (A :type Float%20%28double-precision%29))
  ;[0.15 0.15 0.15 0.5] Timer
  (if (Variables|Default|GetIsRunning)
    (bind _output_get (Variables|Default|SetTotalDeltaSeconds (+ (* A (Variables|Default|GetSpeed)) (Variables|Default|GetTotalDeltaSeconds))))
    (Rendering|Components|TextRender|SetText (Variables|Default|GetTextRender) (Utilities|Text|ToText(String) (Utilities|String|Append (CallFunction|FloattoString00 (Math|Conversions|ToFloat(Integer) (Math|Integer|%(Integer) (Math|Float|Floor (/ _output_get 8.64e+03)) 24))) ":" (CallFunction|FloattoString00 (Math|Conversions|ToFloat(Integer) (Math|Integer|%(Integer) (Math|Float|Floor (/ _output_get 3.6e+02)) 60))) ":" (CallFunction|FloattoString00 (Math|Conversions|ToFloat(Integer) (Math|Float|Floor (Math|Float|%(Float) _output_get 6e+01)))))))))

(event EventPlayAction
  (params (IsPlay :type Boolean))
  (Variables|Default|SetIsRunning IsPlay))

(event EventTick
  (params (DeltaSeconds :type Float%20%28single-precision%29))
  (CallFunction|Run DeltaSeconds))

(fn ConstructionScript)

(fn FloattoString00
  (params (In%20Value :type Float%20%28double-precision%29))
  (return (Utilities|String|Append (Utilities|String|ToString(Integer) (Math|Float|Floor (/ In%20Value 1e+01))) (Utilities|String|ToString(Integer) (Math|Float|Floor (Math|Float|%(Float) In%20Value 1e+01))))))